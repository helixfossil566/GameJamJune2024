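; Interactive locked toy box puzzle that opens to raise a rifle, which becomes pickable after the animation (or from start via SkipCode).
; Use and AlternativeUse route the player's hit component to a four-digit keypad with reset, three tag-identified mode buttons and an intensity knob.
; Each correct setting turns its light good, and all three together trigger Unlock.
; Timelines animate controls, lid and rifle, gating interaction during control and lid motion.
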(event Custom|ModeAnimation
  (bind _current_button (Variables|Default|GetCurrent%20Button))
  (bind _relativelocation (Variables|/Script/Engine.SceneComponent|GetRelativeLocation _current_button))
  ;[0 0.1803 1] Animations
  ;;[0.6667 0.6667 0.6667] Mode Button Animation Settings
  (Variables|Default|SetInteractionEnabled false)
  (Variables|Default|SetCurrentPosition (.y (Variables|/Script/Engine.SceneComponent|GetRelativeLocation (Variables|Default|GetCurrent%20Button))))
  (bind _animation (Timeline|Timeline_2 PlayFromStart)
    (:Update
      (if (Utilities|IsValid _current_button)
        (Transformation|SetRelativeLocation _current_button (Math|Vector|MakeVector (.x _relativelocation) (Math|Float|Lerp (Variables|Default|GetCurrentPosition) (- (Variables|Default|GetCurrentPosition) 0.1) _animation) (.z _relativelocation)) false false)))
    (:Finished
      (Variables|Default|SetInteractionEnabled true))))

(event Custom|ButtonAnimation
  (bind _current_button (Variables|Default|GetCurrent%20Button))
  (bind _relativelocation (Variables|/Script/Engine.SceneComponent|GetRelativeLocation _current_button))
  ;[0 0.1803 1] Animations
  ;;[0.6667 0.6667 0.6667] Button Animation Settings
  (Variables|Default|SetInteractionEnabled false)
  (Variables|Default|SetCurrentPosition (.x (Variables|/Script/Engine.SceneComponent|GetRelativeLocation (Variables|Default|GetCurrent%20Button))))
  (bind _animation (Timeline|Timeline PlayFromStart)
    (:Update
      (if (Utilities|IsValid _current_button)
        (Transformation|SetRelativeLocation _current_button (Math|Vector|MakeVector (Math|Float|Lerp (Variables|Default|GetCurrentPosition) (- (Variables|Default|GetCurrentPosition) 0.1) _animation) (.y _relativelocation) (.z _relativelocation)) false false)))
    (:Finished
      (Variables|Default|SetInteractionEnabled true))))

(event Custom|OpenAnimation
  ;[0 0.1803 1] Animations
  ;;[1 1 1] Open Animation Settings
  (Variables|Default|SetInteractionEnabled false)
  (bind _animation (Timeline|Timeline_3 PlayFromStart)
    (:Update
      (Transformation|SetRelativeRotation (Variables|Default|GetHautToyBox) (Math|Rotator|MakeRotator (* _animation -1.1e+02) 0.0 -1.8e+02) false false))
    (:Finished
      (Variables|Default|SetInteractionEnabled true))))

(event Custom|Correct%20Code%20Sound
  (bind _correctcodesound (Variables|Default|GetCorrectCodeSound))
  ;[1 0 0] Sons
  (Utilities|HM3DSound _correctcodesound false _correctcodesound (Variables|Default|GetDigit_Background) (Variables|Default|GetSoundAttenuation) 0.0))

(event Custom|Button%20Sound
  (bind _emptybutton (Variables|Default|GetEmptyButton))
  (bind _buttonsound (Variables|Default|GetButtonSound))
  (bind _emptybuttonsound (Variables|Default|GetEmptyButtonSound))
  (bind _returnvalue (select _emptybutton _emptybuttonsound _buttonsound))
  ;[1 0 0] Sons
  (Utilities|HM3DSound _returnvalue false _returnvalue (Variables|Default|GetDigit_Background) (Variables|Default|GetSoundAttenuation) 0.0))

(event Custom|WrongScreen
  ;[1 1 1] Digit Screen Settings
  (Utilities|FlowControl|Sequence
    (:then_0
      (Utilities|FlowControl|Delay 0.2)
      (Variables|Default|SetInteractionEnabled false)
      (Utilities|FlowControl|Delay 0.8)
      (Variables|Default|SetInteractionEnabled true))))

(event Custom|Backward%20Knob
  (bind _knob (Variables|Default|GetKnob))
  (bind _relativerotation (Variables|/Script/Engine.SceneComponent|GetRelativeRotation _knob))
  ;[0 0.1803 1] Animations
  ;;[1 1 1] Reverse Knob Animation Settings
  (Variables|Default|SetInteractionEnabled false)
  (bind _animation (Timeline|Timeline_0 PlayFromStart)
    (:Update
      (Transformation|SetRelativeRotation _knob (Math|Rotator|MakeRotator (+ (* _animation 18.0) (Variables|Default|GetCurrentRotation)) (.pitch _relativerotation) (.yaw _relativerotation)) false false)
      (Utilities|FlowControl|Delay 0.25)
      (Variables|Default|SetCurrentRotation (+ (* _animation 18.0) (Variables|Default|GetCurrentRotation))))
    (:Finished
      (Variables|Default|SetInteractionEnabled true))))

(event Custom|ChangeScreen
  ;[1 1 1] Digit Screen Settings
  (bind _output_get (Variables|Default|SetNewScreen (Utilities|Select :Index (- (Variables|Default|GetCurrent_Mode) 1) :Option%200 "/Game/Assets/ToyBox/M_Screen_Mode_1.M_Screen_Mode_1" :Option%201 "/Game/Assets/ToyBox/M_Screen_Mode_2.M_Screen_Mode_2" :Option%202 "/Game/Assets/ToyBox/M_Screen_Mode_3.M_Screen_Mode_3")))
  (Rendering|Material|SetMaterial (Variables|Default|GetDigit_Background) 0 _output_get))

(event Custom|Wrong%20Code%20Sound
  (bind _wrongcodesound (Variables|Default|GetWrongCodeSound))
  ;[1 0 0] Sons
  (Utilities|HM3DSound _wrongcodesound false _wrongcodesound (Variables|Default|GetDigit_Background) (Variables|Default|GetSoundAttenuation) 0.0))

(event Custom|Change%20Light
  (params (Target_Light :type Primitive%20Component%20Object%20Reference) (Light_Value :type Integer))
  ;[1 1 1] Light Settings
  (bind _output_get (Variables|Default|SetNewLight (Utilities|Select :Index Light_Value :Option%200 "/Game/Assets/ToyBox/Light_Good.Light_Good" :Option%201 "/Game/Assets/ToyBox/Light_Wrong.Light_Wrong")))
  (Rendering|Material|SetMaterial Target_Light 0 _output_get))

(event Custom|KnobAnimation
  (bind _knob (Variables|Default|GetKnob))
  (bind _relativerotation (Variables|/Script/Engine.SceneComponent|GetRelativeRotation _knob))
  ;[0 0.1803 1] Animations
  ;;[1 1 1] Knob Animation Settings
  (Variables|Default|SetInteractionEnabled false)
  (bind _animation (Timeline|Timeline_1 PlayFromStart)
    (:Update
      (Transformation|SetRelativeRotation _knob (Math|Rotator|MakeRotator (+ (* _animation -18.0) (Variables|Default|GetCurrentRotation)) (.pitch _relativerotation) (.yaw _relativerotation)) false false)
      (Utilities|FlowControl|Delay 0.25)
      (Variables|Default|SetCurrentRotation (+ (* _animation -18.0) (Variables|Default|GetCurrentRotation))))
    (:Finished
      (Variables|Default|SetInteractionEnabled true))))

(event Custom|DigitScreen
  (bind _currentvalues (Variables|Default|GetCurrentValues))
  (bind _returnvalue (Utilities|Array|LastIndex _currentvalues))
  ;[1 1 1] Digit Screen Settings
  (Rendering|Components|TextRender|SetText (Utilities|Select :Index _returnvalue :Option%200 (Variables|Default|GetDigit_4) :Option%201 (Variables|Default|GetDigit_3) :Option%202 (Variables|Default|GetDigit_2) :Option%203 (Variables|Default|GetDigit_1)) (Utilities|Text|ToText(Integer) (Utilities|Array|Get(acopy) (Variables|Default|GetCurrentValues) _returnvalue))))

(event Custom|Ready%20to%20unlock
  (params (HorrorEvent :type Boolean))
  ;[1 1 1] Lock / Unlock Settings
  (if (Math|Boolean|ANDBoolean (Variables|Default|GetBonCode) (Variables|Default|GetBonMode) (Variables|Default|GetBonneIntensity))
    (CallFunction|Unlock false)))

(event EventAlternativeUse
  (params (HorrorEvent :type Boolean))
  (bind _intensity_light (Variables|Default|GetIntensity_Light))
  ;[1 1 1] Set le bouton sur lequel on a cliqué avec clique gauche ou clique droit
  (Utilities|HMCheckInteraction)
  (bind _asmaster (CallFunction|GetPlayer))
  (Variables|Default|SetCurrent%20Button (Variables|/Game/HorrorEngine/HorrorEngine.HorrorEngine_C|GetHitComponent _asmaster))
  (if (Variables|Default|GetLocked)
    ;[1 1 1] Pressed intensity?
    (if (== (Variables|Default|GetKnob) (Variables|Default|GetCurrent%20Button))
      ;[1 1 1] Knob à fond?
      (if (> (Variables|Default|GetCurrent_Intensity) 0)
        ;[1 1 1] Augmente intensity de 1
        (Variables|Default|SetCurrent_Intensity (- (Variables|Default|GetCurrent_Intensity) 1))
        (CallFunction|BackwardKnob)
        ;[1 1 1] Bonne intensité?
        (if (== (Variables|Default|GetCurrent_Intensity) (Variables|Default|GetTarget_Intensity))
          (CallFunction|ChangeLight _intensity_light)
          (Variables|Default|SetBonneIntensity true)
          (CallFunction|ReadytoUnlock false)
          (else
            (CallFunction|ChangeLight _intensity_light 1)
            (Variables|Default|SetBonneIntensity false)))))))

(event EventBeginPlay
  ;[1 1 1] allow to bypass the code
  (Variables|/Game/FirstPerson/Blueprints/BP_Pickup_Rifle.BP_Pickup_Rifle_C|SetCanBePicked (Variables|Default|GetPickupRifle) (Variables|Default|GetSkipCode)))

(event EventLock
  (params (HorrorEvent :type Boolean))
  ;[1 1 1] Lock / Unlock Settings
  (Variables|Default|SetCurrentValues (Variables|Default|GetResets))
  (CallFunction|WrongCodeSound)
  (Variables|Default|SetLocked true)
  (Variables|Default|SetEmptyButton false))

(event EventUnlock
  (params (HorrorEvent :type Boolean))
  (bind _returnvalue (Utilities|Time|GetWorldDeltaSeconds))
  (bind _pickuprifle (Variables|Default|GetPickupRifle))
  ;[1 1 1] Lock / Unlock Settings
  (CallFunction|OpenAnimation)
  (CallFunction|CorrectCodeSound)
  (Default|CallOpenEventDispatcher)
  (Variables|Default|SetLocked false)
  (Variables|Default|SetEmptyButton true)
  (Utilities|FlowControl|Delay 0.5)
  ;;[1 1 1] Riffle Animation
  (bind (_direction _rotationammount _translationammount) (Timeline|Rase%20the%20gun PlayFromStart) ; it gives a 90° rotation / 10 cm translation
    (:Update
      (Class|Actor|AddActorWorldTransform _pickuprifle (Math|Transform|MakeTransform (* _returnvalue _translationammount (Math|Vector|VectorUp)) (Math|Vector|RotatorfromAxisandAngle "1.000000,0.000000,0.000000" (* _rotationammount _returnvalue)) (Transformation|GetActorScale3D (Variables|Default|GetPickupRifle))) false false)
      (Development|SetHiddeninGame (Variables|Default|GetPlane) false false))
    (:Finished
      (Variables|/Game/FirstPerson/Blueprints/BP_Pickup_Rifle.BP_Pickup_Rifle_C|SetCanBePicked _pickuprifle true) ; the rifle can be picked when the animation\nis over
    )))

(event EventUse
  (params (HorrorEvent :type Boolean))
  (bind _mode_light (Variables|Default|GetMode_Light))
  (bind _intensity_light (Variables|Default|GetIntensity_Light))
  ;[1 1 1] Set le bouton sur lequel on a cliqué avec clique gauche ou clique droit
  (Utilities|HMCheckInteraction)
  (bind _asmaster (CallFunction|GetPlayer))
  (Variables|Default|SetCurrent%20Button (Variables|/Game/HorrorEngine/HorrorEngine.HorrorEngine_C|GetHitComponent _asmaster))
  (if (Variables|Default|GetLocked)
    ;[1 1 1] Pressed intensity?
    (if (== (Variables|Default|GetKnob) (Variables|Default|GetCurrent%20Button))
      ;[1 1 1] Knob à fond?
      (if (< (Variables|Default|GetCurrent_Intensity) 10)
        ;[1 1 1] Augmente intensity de 1
        (Variables|Default|SetCurrent_Intensity (+ (Variables|Default|GetCurrent_Intensity) 1))
        (CallFunction|KnobAnimation)
        ;[1 1 1] Bonne intensité?
        (if (== (Variables|Default|GetCurrent_Intensity) (Variables|Default|GetTarget_Intensity))
          (CallFunction|ChangeLight _intensity_light)
          (Variables|Default|SetBonneIntensity true)
          (CallFunction|ReadytoUnlock false)
          (else
            (CallFunction|ChangeLight _intensity_light 1)
            (Variables|Default|SetBonneIntensity false))))
      (else
        ;[1 1 1] Pressed Reset or Digits?
        (if (== (Variables|Default|GetCurrent%20Button) (Variables|Default|GetBTN_Reset))
          (CallFunction|ButtonAnimation)
          ;[1 1 1] Reset
          (Variables|Default|SetCurrentValues (Variables|Default|GetResets))
          (Utilities|FlowControl|Sequence
            (:then_0
              (Rendering|Components|TextRender|SetText (Variables|Default|GetDigit_1) (Variables|Default|GetReset_Value)))
            (:then_1
              (Rendering|Components|TextRender|SetText (Variables|Default|GetDigit_2) (Variables|Default|GetReset_Value)))
            (:then_2
              (Rendering|Components|TextRender|SetText (Variables|Default|GetDigit_3) (Variables|Default|GetReset_Value)))
            (:then_3
              (Rendering|Components|TextRender|SetText (Variables|Default|GetDigit_4) (Variables|Default|GetReset_Value))
              (CallFunction|ButtonSound)
              (Variables|Default|SetEmptyButton false)
              (CallFunction|Lock false)
              (CallFunction|ChangeLight (Variables|Default|GetCode_Light) 1)))
          (else
            ;[1 1 1] Pressed modes?
            (if (Math|Boolean|ORBoolean (== (Variables|Default|GetCurrent%20Button) (Variables|Default|GetBouton_mode_1)) (== (Variables|Default|GetCurrent%20Button) (Variables|Default|GetBouton_Mode_2)) (== (Variables|Default|GetCurrent%20Button) (Variables|Default|GetBouton_Mode_3)))
              ;[1 1 1] Set Current Mode
              (Variables|Default|SetCurrent_Mode (Math|Conversions|ToInteger(Byte) (Utilities|String|ToString(Name) (Utilities|Array|Get(acopy) (Variables|/Script/Engine.ActorComponent|GetComponentTags (Variables|Default|GetCurrent%20Button))))))
              (CallFunction|ModeAnimation)
              (CallFunction|ButtonSound)
              (CallFunction|ChangeScreen)
              ;[1 1 1] Bon mode?
              (if (== (Variables|Default|GetCurrent_Mode) (Variables|Default|GetTarget_mode))
                (CallFunction|ChangeLight _mode_light)
                (Variables|Default|SetBonMode true)
                (CallFunction|ReadytoUnlock false)
                (else
                  (CallFunction|WrongCodeSound)
                  (CallFunction|ChangeLight _mode_light 1)
                  (Variables|Default|SetBonMode false)))
              (else
                (CallFunction|ButtonAnimation)
                ;[1 1 1] Already Entered 4 Digits?
                (if (>= (Utilities|Array|LastIndex (Variables|Default|GetCurrentValues)) 3)
                  ;[1 1 1] Disable Digital Button Sound
                  (Variables|Default|SetEmptyButton true)
                  (else
                    ;[1 1 1] Calculate Digits
                    (Utilities|Array|Add (Variables|Default|GetCurrentValues) (Math|Conversions|ToInteger(Byte) (Utilities|String|ToString(Name) (Utilities|Array|Get(acopy) (Variables|/Script/Engine.ActorComponent|GetComponentTags (Variables|Default|GetCurrent%20Button))))))
                    (CallFunction|DigitScreen)
                    (Variables|Default|SetEmptyButton false)
                    (CallFunction|ButtonSound)
                    ;[1 1 1] 4 Chiffres entré?
                    (if (== (Utilities|Array|LastIndex (Variables|Default|GetCurrentValues)) 3)
                      ;[1 1 1] Bon code?
                      (if (== (+ (* (Utilities|Array|Get(acopy) (Variables|Default|GetCurrentValues) 3) 1) (* (Utilities|Array|Get(acopy) (Variables|Default|GetCurrentValues) 2) 10) (* (Utilities|Array|Get(acopy) (Variables|Default|GetCurrentValues) 1) 100) (* (Utilities|Array|Get(acopy) (Variables|Default|GetCurrentValues)) 1000)) (Variables|Default|GetCode))
                        (CallFunction|ChangeLight (Variables|Default|GetCode_Light))
                        (Variables|Default|SetBonCode true)
                        (CallFunction|ReadytoUnlock false)
                        (else
                          (CallFunction|WrongCodeSound)
                          (CallFunction|ChangeLight (Variables|Default|GetCode_Light) 1)
                          (Variables|Default|SetBonCode false))))))))))))))

(fn ConstructionScript
  (|CallParentFunction)
  (CallFunction|PlayRate (Variables|Default|GetWarningTimeline) (Variables|Default|GetDetectionWarningDuration%28Sec%29)))